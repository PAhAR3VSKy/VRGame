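; Paper airplane quest object that motion controllers can pick up and drop, with physics that responds to time stopping.
; Pickup disables physics on the Box and attaches the root to the controller; Drop detaches it and simulates physics only while the Time flag is true.
; When dropped in stopped time, it stores a scaled-down Box velocity in StopMotion.
; TimeStoped only clears the flag, while TimeComein sets it, re-enables physics and adds the stored velocity.
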(event EventTimeStoped
  (Variables|Default|SetTime false))

(event EventPickup
  (params (AttachTo :type Scene%20Component%20Object%20Reference))
  (Physics|SetSimulatePhysics (Variables|Default|GetBox) false)
  (Transformation|AttachComponentToComponent (VehicleSound|GetRootComponent) AttachTo "None" "KeepWorld" "KeepWorld" "KeepWorld" false))

(event EventDrop
  (bind _box (Variables|Default|GetBox))
  (bind _time (Variables|Default|GetTime))
  (Physics|SetSimulatePhysics _box _time)
  (Transformation|DetachFromActor "KeepWorld" "KeepWorld" "KeepWorld")
  (Development|PrintString (Utilities|String|ToString(Boolean) _time))
  (if (not _time)
    (bind _returnvalue (Physics|GetPhysicsLinearVelocity _box "None"))
    (Variables|Default|SetStop%20Motion (/ _returnvalue 1e+04))))

(event EventTimeComein
  (bind _box (Variables|Default|GetBox))
  (Variables|Default|SetTime true)
  (Physics|SetSimulatePhysics _box true)
  (Class|PrimitiveComponent|SetAllPhysicsLinearVelocity _box (Variables|Default|GetStop%20Motion) true))

(fn ConstructionScript)