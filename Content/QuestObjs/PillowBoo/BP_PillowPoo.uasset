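; BP_PillowPoo is a physics pillow prop that motion controllers can pick up and drop, with time-stop and growth behavior.
; Pickup attaches it with physics off; Drop detaches it, simulating only if time runs.
; Drops during stopped time store scaled-down velocity, which TimeComein adds when re-enabling physics.
; GroovOn steps up Z scale on a delay loop, which ends only at a threshold while the Groo flag is set.
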(event Custom|GroovOn
  (bind _returnvalue (Transformation|GetActorScale3D))
  (bind _returnvalue_2 (+ (.z _returnvalue) 0.05))
  (Variables|Default|SetGroo true)
  (Transformation|SetActorScale3D (Math|Vector|MakeVector (.x _returnvalue) (.y _returnvalue) _returnvalue_2) :!label _label)
  (if (not (and (>= _returnvalue_2 0.2) (Variables|Default|GetGroo)))
    (Utilities|FlowControl|Delay 0.3)
    (goto _label)))

(event Custom|GroovOff
  (Variables|Default|SetGroo false))

(event EventBeginPlay)

(event Collision|EventActorBeginOverlap
  (params (OtherActor :type Actor%20Object%20Reference)))

(event EventTimeStoped
  (Variables|Default|SetTime false))

(event EventPickup
  (params (AttachTo :type Scene%20Component%20Object%20Reference))
  (Physics|SetSimulatePhysics (Variables|Debug|GetStaticMeshComponent) false)
  (Transformation|AttachComponentToComponent (VehicleSound|GetRootComponent) AttachTo "None" "KeepWorld" "KeepWorld" "KeepWorld" false))

(event EventTick
  (params (DeltaSeconds :type Float%20%28single-precision%29)))

(event EventDrop
  (bind _time (Variables|Default|GetTime))
  (bind _staticmeshcomponent (Variables|Debug|GetStaticMeshComponent))
  (Physics|SetSimulatePhysics _staticmeshcomponent _time)
  (Transformation|DetachFromActor "KeepWorld" "KeepWorld" "KeepWorld")
  (Development|PrintString (Utilities|String|ToString(Boolean) _time))
  (if (not _time)
    (bind _returnvalue (Physics|GetPhysicsLinearVelocity _staticmeshcomponent "None"))
    (Variables|Default|SetStop%20Motion (/ _returnvalue 1e+04))))

(event EventTimeComein
  (bind _staticmeshcomponent (Variables|Debug|GetStaticMeshComponent))
  (Variables|Default|SetTime true)
  (Physics|SetSimulatePhysics _staticmeshcomponent true)
  (Class|PrimitiveComponent|SetAllPhysicsLinearVelocity _staticmeshcomponent (Variables|Default|GetStop%20Motion) true))

(fn ConstructionScript)