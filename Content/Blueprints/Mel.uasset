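; Mel is a grabbable VR actor that draws on Doska boards like a piece of chalk.
; Pickup and Drop toggle physics and attach it to or detach it from the motion controller component.
; Overlaps on the mesh or Sphere toggle IsDraw; while set, Tick prints a debug vector and line-traces briefly from the Sphere along its absolute, flattened forward vector.
; Doska hits pass their collision UV to DrawOnDoska.
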(event OnComponentBeginOverlap(Sphere)
  (params (OverlappedComponent :type Primitive%20Component%20Object%20Reference) (OtherActor :type Actor%20Object%20Reference) (OtherComp :type Primitive%20Component%20Object%20Reference) (OtherBodyIndex :type Integer) (bFromSweep :type Boolean) (SweepResult :type Hit%20Result%20Structure%20%28by%20ref%29))
  (Variables|Default|Setis%20Draw true))

(event OnComponentBeginOverlap(StaticMeshComponent)
  (params (OverlappedComponent :type Primitive%20Component%20Object%20Reference) (OtherActor :type Actor%20Object%20Reference) (OtherComp :type Primitive%20Component%20Object%20Reference) (OtherBodyIndex :type Integer) (bFromSweep :type Boolean) (SweepResult :type Hit%20Result%20Structure%20%28by%20ref%29))
  (Variables|Default|Setis%20Draw true))

(event OnComponentEndOverlap(StaticMeshComponent)
  (params (OverlappedComponent :type Primitive%20Component%20Object%20Reference) (OtherActor :type Actor%20Object%20Reference) (OtherComp :type Primitive%20Component%20Object%20Reference) (OtherBodyIndex :type Integer))
  (Variables|Default|Setis%20Draw false))

(event OnComponentEndOverlap(Sphere)
  (params (OverlappedComponent :type Primitive%20Component%20Object%20Reference) (OtherActor :type Actor%20Object%20Reference) (OtherComp :type Primitive%20Component%20Object%20Reference) (OtherBodyIndex :type Integer))
  (Variables|Default|Setis%20Draw false))

(event EventBeginPlay)

(event Collision|EventActorBeginOverlap
  (params (OtherActor :type Actor%20Object%20Reference)))

(event EventPickup
  (params (AttachTo :type Scene%20Component%20Object%20Reference))
  (Physics|SetSimulatePhysics (Variables|Debug|GetStaticMeshComponent) false)
  (Transformation|AttachComponentToComponent (VehicleSound|GetRootComponent) AttachTo "None" "KeepWorld" "KeepWorld" "KeepWorld" false))

(event EventTick
  (params (DeltaSeconds :type Float%20%28single-precision%29))
  (bind _sphere (Variables|Default|GetSphere))
  (bind _returnvalue (Transformation|GetWorldLocation _sphere))
  (bind _returnvalue_2 (Math|Vector|GetForwardVector _sphere))
  (bind _returnvalue_3 (Math|Vector|VectorGetAbs _returnvalue_2))
  (bind _returnvalue_4 (Class|KismetMathLibrary|VectorNormal2D _returnvalue_3 0.0001))
  (bind _returnvalue_5 (* _returnvalue_4 -2.0))
  (if (Variables|Default|Getis%20Draw)
    (Development|PrintString (Utilities|String|ToString(Vector) _returnvalue_5))
    (bind (_outhit _returnvalue_6) (Collision|LineTraceByChannel _returnvalue (+ (* _returnvalue_5 -7.0) _returnvalue) "TraceTypeQuery1" true 0 "None"))
    (if _returnvalue_6
      (bind _asdoska (Utilities|Casting|CastToDoska (.HitActor (Collision|BreakHitResult _outhit))))
      (Default|DrawonDoska _asdoska (.UV (Class|GameplayStatics|FindCollisionUV _outhit))))))

(event EventDrop
  (Physics|SetSimulatePhysics (Variables|Debug|GetStaticMeshComponent) true)
  (Transformation|DetachFromActor "KeepWorld" "KeepWorld" "KeepWorld"))

(fn ConstructionScript)