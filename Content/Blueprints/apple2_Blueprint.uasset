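; Pickup-able apple actor that BP_MotionController can attach and drop, with support for a time-stop mechanic.
; Drop simulates physics only while Time is true; otherwise it stores a heavily scaled-down velocity in StopMotion.
; TimeStoped only clears the Time flag, while TimeComein sets it, re-enables physics and adds StopMotion back.
; Overlaps toggle IsDraw, but the line-trace logic for drawing on a Doska is unconnected and never runs.
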(event OnComponentBeginOverlap(StaticMeshComponent)
  (params (OverlappedComponent :type Primitive%20Component%20Object%20Reference) (OtherActor :type Actor%20Object%20Reference) (OtherComp :type Primitive%20Component%20Object%20Reference) (OtherBodyIndex :type Integer) (bFromSweep :type Boolean) (SweepResult :type Hit%20Result%20Structure%20%28by%20ref%29))
  (Variables|Default|SetisDraw true))

(event OnComponentEndOverlap(StaticMeshComponent)
  (params (OverlappedComponent :type Primitive%20Component%20Object%20Reference) (OtherActor :type Actor%20Object%20Reference) (OtherComp :type Primitive%20Component%20Object%20Reference) (OtherBodyIndex :type Integer))
  (Variables|Default|SetisDraw false))

(event EventBeginPlay)

(event Collision|EventActorBeginOverlap
  (params (OtherActor :type Actor%20Object%20Reference)))

(event EventTimeStoped
  (Development|PrintString "APPLE stop" true true "(R=1.000000,G=0.131410,B=0.211110,A=1.000000)")
  (Variables|Default|Settime false))

(event EventPickup
  (params (AttachTo :type Scene%20Component%20Object%20Reference))
  (Physics|SetSimulatePhysics (Variables|Debug|GetStaticMeshComponent) false)
  (Transformation|AttachComponentToComponent (VehicleSound|GetRootComponent) AttachTo "None" "KeepWorld" "KeepWorld" "KeepWorld" false))

(event EventTick
  (params (DeltaSeconds :type Float%20%28single-precision%29)))

(event EventDrop
  (bind _time (Variables|Default|Gettime))
  (bind _staticmeshcomponent (Variables|Debug|GetStaticMeshComponent))
  (Physics|SetSimulatePhysics _staticmeshcomponent _time)
  (Transformation|DetachFromActor "KeepWorld" "KeepWorld" "KeepWorld")
  (Development|PrintString "APPLE DROPED")
  (if (not _time)
    (bind _returnvalue (Physics|GetPhysicsLinearVelocity _staticmeshcomponent "None"))
    (Variables|Default|Setstop_motion (/ _returnvalue 1e+04))))

(event EventTimeComein
  (bind _staticmeshcomponent (Variables|Debug|GetStaticMeshComponent))
  (Development|PrintString "APPLe go" true true "(R=1.000000,G=0.017294,B=0.096967,A=1.000000)" 6e+01)
  (Variables|Default|Settime true)
  (Physics|SetSimulatePhysics _staticmeshcomponent true)
  (Class|PrimitiveComponent|SetAllPhysicsLinearVelocity _staticmeshcomponent (Variables|Default|Getstop_motion) true))

(fn ConstructionScript)