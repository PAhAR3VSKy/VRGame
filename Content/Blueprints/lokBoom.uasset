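; lokBoom is a VR pickup Actor that BP_MotionController can grab and drop.
; Pickup uses the IsHand flag as a toggle: when true it shows the Clome component, disables its physics and attaches it to the supplied parent, otherwise it runs the drop logic.
; Drop re-enables physics, detaches the Actor rather than the attached component, and sets IsHand back to true.
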(event EventBeginPlay)

(event Collision|EventActorBeginOverlap
  (params (OtherActor :type Actor%20Object%20Reference)))

(event EventTick
  (params (DeltaSeconds :type Float%20%28single-precision%29)))

(event EventPickup
  (params (AttachTo :type Scene%20Component%20Object%20Reference))
  (bind _clome (Variables|Default|Getclome))
  (if (Variables|Default|GetisHand)
    (Rendering|SetVisibility _clome true false)
    (Physics|SetSimulatePhysics _clome false)
    (Transformation|AttachComponentToComponent _clome AttachTo "None" "KeepWorld" "KeepWorld" "KeepWorld" false)
    (Variables|Default|SetisHand false)
    (else
      (Physics|SetSimulatePhysics (Variables|Default|Getclome) true)
      (Transformation|DetachFromActor "KeepWorld" "KeepWorld" "KeepWorld")
      (Variables|Default|SetisHand true))))

(event EventDrop
  (Physics|SetSimulatePhysics (Variables|Default|Getclome) true)
  (Transformation|DetachFromActor "KeepWorld" "KeepWorld" "KeepWorld")
  (Variables|Default|SetisHand true))

(fn ConstructionScript)