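; Banana_BP is a banana prop that a VR motion controller picks up and drops, with behavior tied to a time-stop state.
; Pickup disables physics and attaches it to the given component, while Drop detaches it and simulates physics only if time is running.
; A drop during stopped time stores a heavily scaled-down velocity, which TimeComein adds back when it re-enables physics.
; TimeStoped only clears the time flag.
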(event EventBeginPlay)

(event Collision|EventActorBeginOverlap
  (params (OtherActor :type Actor%20Object%20Reference)))

(event EventTimeStoped
  (Variables|Default|SetTime false))

(event EventPickup
  (params (AttachTo :type Scene%20Component%20Object%20Reference))
  (Physics|SetSimulatePhysics (Variables|Default|GetStaticMesh) false)
  (Transformation|AttachComponentToComponent (VehicleSound|GetRootComponent) AttachTo "None" "KeepWorld" "KeepWorld" "KeepWorld" false))

(event EventTick
  (params (DeltaSeconds :type Float%20%28single-precision%29)))

(event EventDrop
  (bind _time (Variables|Default|GetTime))
  (bind _staticmesh (Variables|Default|GetStaticMesh))
  (Physics|SetSimulatePhysics _staticmesh _time)
  (Transformation|DetachFromActor "KeepWorld" "KeepWorld" "KeepWorld")
  (Development|PrintString (Utilities|String|ToString(Boolean) _time))
  (if (not _time)
    (bind _returnvalue (Physics|GetPhysicsLinearVelocity _staticmesh "None"))
    (Variables|Default|SetStop%20Motion (/ _returnvalue 1e+04))))

(event EventTimeComein
  (bind _staticmesh (Variables|Default|GetStaticMesh))
  (Variables|Default|SetTime true)
  (Physics|SetSimulatePhysics _staticmesh true)
  (Class|PrimitiveComponent|SetAllPhysicsLinearVelocity _staticmesh (Variables|Default|GetStop%20Motion) true))

(fn ConstructionScript)