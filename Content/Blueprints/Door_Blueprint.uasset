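; Door actor that swings its LeftDoor component while something overlaps it.
; Overlap sets a DoorTouch flag, and Tick then adds a fixed yaw step each frame, not scaled by delta time, signed by ToOpen.
; Ending the overlap stops rotation and negates ToOpen, so the next touch swings the opposite way.
; Motion-controller Pickup and Drop events are empty, with their attach, detach and physics logic left unconnected.
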(event OnComponentBeginOverlap(leftDoor)
  (params (OverlappedComponent :type Primitive%20Component%20Object%20Reference) (OtherActor :type Actor%20Object%20Reference) (OtherComp :type Primitive%20Component%20Object%20Reference) (OtherBodyIndex :type Integer) (bFromSweep :type Boolean) (SweepResult :type Hit%20Result%20Structure%20%28by%20ref%29))
  (Variables|Default|Setdoor_touch true))

(event OnComponentEndOverlap(leftDoor)
  (params (OverlappedComponent :type Primitive%20Component%20Object%20Reference) (OtherActor :type Actor%20Object%20Reference) (OtherComp :type Primitive%20Component%20Object%20Reference) (OtherBodyIndex :type Integer))
  (Variables|Default|Setdoor_touch false)
  (Variables|Default|SettoOpen (* (Variables|Default|GettoOpen) -1)))

(event EventBeginPlay)

(event Collision|EventActorBeginOverlap
  (params (OtherActor :type Actor%20Object%20Reference)))

(event EventTick
  (params (DeltaSeconds :type Float%20%28single-precision%29))
  (if (Variables|Default|Getdoor_touch)
    (Transformation|AddLocalRotation (Variables|Default|GetleftDoor) (Math|Rotator|MakeRotator 0.0 0.0 (* (Variables|Default|GettoOpen) 0.7)) false false)))

(event EventPickup
  (params (AttachTo :type Scene%20Component%20Object%20Reference)))

(event EventDrop)

(fn ConstructionScript)